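; Plant enemy that fires BolaPlanta_BP projectiles and can be killed by damage or by a jump.
; Hearing a noise through PawnSensing starts a looping timer that flags the anim Blueprint as attacking and spawns each projectile.
; Seeing a pawn only sets PlantaShoot, which is cleared after each shot but never read here.
; Lethal damage destroys it with a sound, while the jump Death event first scales the capsule via a timeline.
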(event OnHearNoise(PawnSensing)
  (params (Instigator :type Pawn%20Object%20Reference) (Location :type Vector%20%28by%20ref%29 :default "0, 0, 0") (Volume :type Float%20%28single-precision%29))
  (Utilities|Time|SetTimerbyEvent (delegate Custom|FireShoot) 2.0 true))

(event OnSeePawn(PawnSensing)
  (params (Pawn :type Pawn%20Object%20Reference))
  (Variables|Default|SetPlantaShoot true))

(event Custom|Death
  ;[1 1 1] Death By Jump
  (Utilities|FlowControl|DoOnce false
    (:Completed
      (bind _newtrack_0 (Timeline|ScalePlant PlayFromStart)
        (:Update
          (Transformation|SetWorldScale3D (Variables|Collision|GetCapsuleComponent) _newtrack_0))
        (:Finished
          (Utilities|FlowControl|Delay 1.0)
          (Audio|PlaySound2D "/Game/SFX/PlantaSounds/plantamuerte.plantamuerte" 1.0 1.0 0.0 0 0)
          (Actor|DestroyActor))))))

(event Custom|FireShoot
  (bind _asplanta_ab (Utilities|Casting|CastToPlanta_AB (Components|SkeletalMesh|GetAnimInstance (Variables|Character|GetMesh))))
  (Variables|/Game/Blueprints/Planta/Planta_AB.Planta_AB_C|SetIsAttacking? _asplanta_ab true)
  (Game|SpawnActorfromClass "/Game/Blueprints/Planta/BolaPlanta_BP.BolaPlanta_BP_C" (Transformation|GetSocketTransform (Variables|Collision|GetCapsuleComponent) "BolaSocket" "RTS_World") "Undefined" 0 0)
  (Utilities|FlowControl|Delay 1.0)
  (Variables|Default|SetPlantaShoot false))

(event Game|Damage|EventAnyDamage
  (params (Damage :type Float%20%28single-precision%29) (DamageType :type Damage%20Type%20Object%20Reference) (InstigatedBy :type Controller%20Object%20Reference) (DamageCauser :type Actor%20Object%20Reference))
  (bind _output_get (Variables|Default|SetVidaPlanta (- (Variables|Default|GetVidaPlanta) Damage)))
  (if (<= _output_get 0.0)
    (Audio|PlaySound2D "/Game/SFX/PlantaSounds/plantamuerte.plantamuerte" 1.0 1.0 0.0 0 0)
    (Utilities|FlowControl|Delay 0.2)
    (Actor|DestroyActor)))

(event EventBeginPlay)

(fn ConstructionScript)