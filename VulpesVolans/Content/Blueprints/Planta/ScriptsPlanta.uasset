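; Plant enemy character that moves toward the player and fires projectiles once it spots them.
; Pawn sensing detects the player, sets PlantaShoot and starts AI movement; the reset branch is unreachable, so shooting never switches off.
; A three-second Delay loop from BeginPlay sets the animation blueprint's attack flag and, while shooting, spawns BolaPlanta_BP at the capsule's BolaSocket transform.
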(event OnSeePawn(PawnSensing)
  (params (Pawn :type Pawn%20Object%20Reference))
  (if true
    (bind _asvv_player_bp (Utilities|Casting|CastToVV_PlayerBP Pawn))
    (Variables|Default|SetPlantaShoot true)
    (AI|AIMoveTo 0 "0, 0, 0" _asvv_player_bp 5.0 false)
    (else
      (Variables|Default|SetPlantaShoot false))))

(event EventBeginPlay
  (if (Variables|Default|GetPlantaShoot) :!label _label
    (bind _asplanta_ab (Utilities|Casting|CastToPlanta_AB (Components|SkeletalMesh|GetAnimInstance (Variables|Character|GetMesh))))
    (Variables|/Game/Blueprints/Planta/Planta_AB.Planta_AB_C|SetIsAttacking? _asplanta_ab true)
    (Game|SpawnActorfromClass "/Game/Blueprints/Planta/BolaPlanta_BP.BolaPlanta_BP_C" (Transformation|GetSocketTransform (Variables|Collision|GetCapsuleComponent) "BolaSocket" "RTS_World") "Undefined" 0 0)
    (Utilities|FlowControl|Delay 3.0)
    (goto _label)
    (else
      (bind _asplanta_ab_2 (Utilities|Casting|CastToPlanta_AB (Components|SkeletalMesh|GetAnimInstance (Variables|Character|GetMesh))))
      (Variables|/Game/Blueprints/Planta/Planta_AB.Planta_AB_C|SetIsAttacking? _asplanta_ab_2 false)
      (Utilities|FlowControl|Delay 3.0)
      (goto _label))))

(fn ConstructionScript)