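; BP_MuroInvisible is an invisible wall actor that removes itself once the gem goal is reached.
; Every Tick it casts the game mode to ThirdPersonGameMode and destroys itself when the total gem count equals three.
; An unconnected, never-run branch holds an alternative check against the gem count on VV_PlayerBP.
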(event EventBeginPlay)

(event Collision|EventActorBeginOverlap
  (params (OtherActor :type Actor%20Object%20Reference)))

(event EventTick
  (params (DeltaSeconds :type Float%20%28single-precision%29))
  (bind _asthird_person_game_mode (Utilities|Casting|CastToThirdPersonGameMode (Game|GetGameMode)))
  (bind _output_get (Variables|Default|SetAs%20Third%20Person%20Game%20Mode _asthird_person_game_mode))
  (if (== (Variables|/Game/Blueprints/ThirdPersonGameMode.ThirdPersonGameMode_C|GetNumeroGemasTotales _output_get) 3)
    (Actor|DestroyActor)))

(fn ConstructionScript)