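; DisparoMosquito_BP is a mosquito enemy projectile that damages the VV player character on contact.
; Overlap on its ball collider subtracts health from VV_PlayerBP, plays a shot sound and destroys the projectile.
; If the player's health reaches zero or below, it also destroys the player and plays a death sound.
; Projectiles that hit nothing destroy themselves after a one-minute lifetime.
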(event OnComponentBeginOverlap(BolaCollider)
  (params (OverlappedComponent :type Primitive%20Component%20Object%20Reference) (OtherActor :type Actor%20Object%20Reference) (OtherComp :type Primitive%20Component%20Object%20Reference) (OtherBodyIndex :type Integer) (bFromSweep :type Boolean) (SweepResult :type Hit%20Result%20Structure%20%28by%20ref%29))
  (bind _asvv_player_bp (Utilities|Casting|CastToVV_PlayerBP OtherActor))
  (bind _output_get (Variables|/Game/Blueprints/VV/VV_PlayerBP.VV_PlayerBP_C|SetVidaVV _asvv_player_bp (- (Variables|/Game/Blueprints/VV/VV_PlayerBP.VV_PlayerBP_C|GetVidaVV _asvv_player_bp) 25.1)))
  (Audio|PlaySound2D "/Game/SFX/MosquitoSounds/disparomosquito.disparomosquito" 1.0 1.0 0.0 0 0)
  (Actor|DestroyActor)
  (if (<= _output_get 0.0)
    (Actor|DestroyActor _asvv_player_bp)
    (Audio|PlaySound2D "/Game/SFX/VVSounds/MuertePersonaje__1_.MuertePersonaje__1_" 1.0 1.0 0.0 0 0)))

(event EventBeginPlay
  (Utilities|FlowControl|Delay 6e+01)
  (Actor|DestroyActor))

(fn ConstructionScript)