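; Base sword Blueprint that instantly kills plant, mosquito and cactus enemies it touches.
; SwordActive switches the sword collider to an overlap-all collision profile, and SwordDeactive disables its collision.
; On overlap it ignores its owner, then runs a cast chain over the three enemy classes, playing that enemy's death sound in 2D before destroying the actor.
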(event OnComponentBeginOverlap(SwordCollider)
  (params (OverlappedComponent :type Primitive%20Component%20Object%20Reference) (OtherActor :type Actor%20Object%20Reference) (OtherComp :type Primitive%20Component%20Object%20Reference) (OtherBodyIndex :type Integer) (bFromSweep :type Boolean) (SweepResult :type Hit%20Result%20Structure%20%28by%20ref%29))
  (if (!= OtherActor (Components|GetOwner))
    (bind _asplanta_enemy_bp (Utilities|Casting|CastToPlantaEnemy_BP OtherActor)
      (:then
        (Audio|PlaySound2D "/Game/SFX/PlantaSounds/plantamuerte.plantamuerte" 1.0 1.0 0.0 0 0)
        (Actor|DestroyActor _asplanta_enemy_bp))
      (:CastFailed
        (bind _asmosquito_enemy_bp (Utilities|Casting|CastToMosquitoEnemy_BP OtherActor)
          (:then
            (Audio|PlaySound2D "/Game/SFX/MosquitoSounds/MosquitoMuerte.MosquitoMuerte" 1.0 1.0 0.0 0 0)
            (Actor|DestroyActor _asmosquito_enemy_bp))
          (:CastFailed
            (bind _ascactus (Utilities|Casting|CastToCactus OtherActor))
            (Audio|PlaySound2D "/Game/Blueprints/Cactus/cactusmuere.cactusmuere" 1.0 1.0 0.0 0 0)
            (Actor|DestroyActor _ascactus)))))))

(event Custom|SwordActive
  (Collision|SetCollisionProfileName (Variables|Default|GetSwordCollider) "OverlapAllDynamic" true :!class /Script/Engine.PrimitiveComponent))

(event Custom|SwordDeactive
  (Collision|SetCollisionEnabled (Variables|Default|GetSwordCollider) "NoCollision"))

(fn ConstructionScript)