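; DamageState is an anim notify state that marks the window in a player animation during which the sword is active.
; On begin and end, it casts the mesh owner to VV_PlayerBP and its child actor to BaseSword_BP.
; It calls SwordActive when the window opens and SwordDeactive when it closes, doing nothing if either cast fails.
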(fn ReceivedNotifyBegin
  (params (MeshComp :type Skeletal%20Mesh%20Component%20Object%20Reference) (Animation :type Anim%20Sequence%20Base%20Object%20Reference) (TotalDuration :type Float%20%28single-precision%29))
  (bind _asvv_player_bp (Utilities|Casting|CastToVV_PlayerBP (Components|GetOwner MeshComp)))
  (bind _asbase_sword_bp (Utilities|Casting|CastToBaseSword_BP (Variables|/Script/Engine.ChildActorComponent|GetChildActor (Variables|/Game/Blueprints/VV/VV_PlayerBP.VV_PlayerBP_C|GetChildActor _asvv_player_bp))))
  (Default|SwordActive _asbase_sword_bp)
  (return false))

(fn ReceivedNotifyEnd
  (params (MeshComp :type Skeletal%20Mesh%20Component%20Object%20Reference) (Animation :type Anim%20Sequence%20Base%20Object%20Reference))
  (bind _asvv_player_bp (Utilities|Casting|CastToVV_PlayerBP (Components|GetOwner MeshComp)))
  (bind _asbase_sword_bp (Utilities|Casting|CastToBaseSword_BP (Variables|/Script/Engine.ChildActorComponent|GetChildActor (Variables|/Game/Blueprints/VV/VV_PlayerBP.VV_PlayerBP_C|GetChildActor _asvv_player_bp))))
  (Default|SwordDeactive _asbase_sword_bp)
  (return false))